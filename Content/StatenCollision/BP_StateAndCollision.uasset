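; BP_StateAndCollision is an actor that reports whether something hit it from behind or from the front.
; On a capsule hit, it flattens the arrow's forward vector and the direction to the other actor, then uses their dot product to choose "Stealth Hit" or "Hit From Front".
; A ShowHit event displays that text for one second, with a DoOnce gate blocking repeats until it hides again.
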(event OnComponentHit(Capsule)
  (params (HitComponent :type Primitive%20Component%20Object%20Reference) (OtherActor :type Actor%20Object%20Reference) (OtherComp :type Primitive%20Component%20Object%20Reference) (NormalImpulse :type Vector :default "0, 0, 0") (Hit :type Hit%20Result%20Structure%20%28by%20ref%29))
  (bind _returnvalue (Transformation|GetActorLocation OtherActor))
  (bind _arrow (Variables|Default|GetArrow))
  (bind _arrow_2 (Variables|Default|GetArrow))
  (bind _returnvalue_2 (Transformation|GetWorldLocation _arrow))
  (bind _returnvalue_3 (Transformation|GetWorldRotation _arrow_2))
  (bind _returnvalue_4 (Math|Vector|GetForwardVector _returnvalue_3))
  (bind _returnvalue_5 (- _returnvalue _returnvalue_2))
  (CallFunction|ShowHit (select (< (Math|Vector|DotProduct (Math|Vector|MakeVector (.x _returnvalue_4) (.y _returnvalue_4) 0.0) (Math|Vector|Normalize (Math|Vector|MakeVector (.x _returnvalue_5) (.y _returnvalue_5) 0.0))) 0.0) "Stealth Hit" "Hit From Front")))

(event Custom|Show%20Hit
  (params (Show%20Text :type Text))
  (bind _showhittext (Variables|Default|GetShowHitText))
  (Utilities|FlowControl|DoOnce false :!label _label
    (:Completed
      (Rendering|Components|TextRender|SetText _showhittext Show%20Text)
      (Rendering|SetVisibility _showhittext true false)
      (Utilities|FlowControl|Delay 1.0)
      (Rendering|SetVisibility (Variables|Default|GetShowHitText) false false)
      (goto _label Reset))))

(event EventBeginPlay
  (Rendering|SetVisibility (Variables|Default|GetShowHitText) false false))

(event Collision|EventActorBeginOverlap
  (params (OtherActor :type Actor%20Object%20Reference)))

(event EventTick
  (params (DeltaSeconds :type Float%20%28single-precision%29)))

(fn ConstructionScript)
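; BP_Interpolation is an elevator actor that moves between a ground floor and a first floor.
; Overlapping its Box trigger runs a FlipFlop that alternately sets TargetFloor to FirstFloor or GroundFloor.
; Each Tick, the Elevator component lerps its relative location toward TargetFloor using DeltaSeconds as alpha, giving an eased approach that stops updating once nearly there.
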(event OnComponentBeginOverlap(Box)
  (params (OverlappedComponent :type Primitive%20Component%20Object%20Reference) (OtherActor :type Actor%20Object%20Reference) (OtherComp :type Primitive%20Component%20Object%20Reference) (OtherBodyIndex :type Integer) (bFromSweep :type Boolean) (SweepResult :type Hit%20Result%20Structure%20%28by%20ref%29))
  (Utilities|FlowControl|FlipFlop
    (:A
      (Variables|Default|SetTargetFloor (Variables|Default|GetFirstFloor)))
    (:B
      (Variables|Default|SetTargetFloor (Variables|Default|GetGroundFloor)))))

(event EventBeginPlay)

(event Collision|EventActorBeginOverlap
  (params (OtherActor :type Actor%20Object%20Reference)))

(event EventTick
  (params (DeltaSeconds :type Float%20%28single-precision%29))
  (bind _elevator (Variables|Default|GetElevator))
  (if (not (Utilities|Operators|EqualEqual (Variables|/Script/Engine.SceneComponent|GetRelativeLocation (Variables|Default|GetElevator)) (Variables|Default|GetTargetFloor) 0.05))
    (Transformation|SetRelativeLocation _elevator (Math|Vector|Lerp(Vector) (Variables|/Script/Engine.SceneComponent|GetRelativeLocation _elevator) (Variables|Default|GetTargetFloor) DeltaSeconds) false false)))

(fn ConstructionScript)
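; BP_Intersection is an actor whose Table component spins while the player is nearby.
; Each Tick finds and caches the BP_ThirdPersonCharacter if needed, looping back to the validity check, then tests proximity.
; DetectPresence compares squared horizontal distance, via a dot product ignoring Z, against DetectionDistance squared.
; The result sets CurrentSwitchStatus, which gates a constant-speed, delta-time-scaled local yaw rotation of the Table.
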(event Custom|SetPlayer
  (bind _returnvalue (Actor|GetActorOfClass "/Game/ThirdPerson/Blueprints/BP_ThirdPersonCharacter.BP_ThirdPersonCharacter_C"))
  (Variables|Default|SetPlayer _returnvalue))

(event Custom|Detect%20Presence
  (bind _returnvalue (Transformation|GetActorLocation))
  (bind _player (Variables|Default|GetPlayer))
  (bind _detectiondistance (Variables|Default|GetDetectionDistance))
  (bind _returnvalue_2 (Transformation|GetActorLocation _player))
  (bind _returnvalue_3 (- (Math|Vector|MakeVector (.x _returnvalue) (.y _returnvalue) 0.0) (Math|Vector|MakeVector (.x _returnvalue_2) (.y _returnvalue_2) 0.0)))
  (CallFunction|ToggleTable (<= (Math|Vector|DotProduct _returnvalue_3 _returnvalue_3) (* _detectiondistance _detectiondistance))))

(event Custom|ToggleTable
  (params (Switch :type Boolean))
  (if (not (== Switch (Variables|Default|GetCurrentSwitchStatus)))
    (Variables|Default|SetCurrentSwitchStatus Switch)))

(event Custom|RotateTable
  (params (DeltaTime :type Float%20%28double-precision%29))
  (Transformation|AddLocalRotation (Variables|Default|GetTable) (Math|Rotator|MakeRotator 0.0 0.0 (* 5e+01 DeltaTime)) false false))

(event EventBeginPlay)

(event Collision|EventActorBeginOverlap
  (params (OtherActor :type Actor%20Object%20Reference)))

(event EventTick
  (params (DeltaSeconds :type Float%20%28single-precision%29))
  (Utilities|IsValid (Variables|Default|GetPlayer) :!label _label
    (:Is%20Valid
      (CallFunction|DetectPresence)
      (if (Variables|Default|GetCurrentSwitchStatus)
        (CallFunction|RotateTable DeltaSeconds)))
    (:Is%20Not%20Valid
      (CallFunction|SetPlayer)
      (goto _label))))

(fn ConstructionScript)